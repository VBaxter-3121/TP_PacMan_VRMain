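; A VR rhythm-game dance note that slides in one of four directions and reports a hit or miss to its dance machine.
; On BeginPlay it sets a direction-based arrow mesh, with Up and Down meshes swapped, and plays a timeline meant to lerp it along the actor's axes.
; Overlap with a DanceHand-tagged component counts as a hit, timeline completion as a miss; a resolved flag prevents double counting before destruction.
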(event OnComponentBeginOverlap(NoteHitBox)
  (params (OverlappedComponent :type Primitive%20Component%20Object%20Reference) (OtherActor :type Actor%20Object%20Reference) (OtherComp :type Primitive%20Component%20Object%20Reference) (OtherBodyIndex :type Integer) (bFromSweep :type Boolean) (SweepResult :type Hit%20Result%20Structure%20%28by%20ref%29))
  (bind _dancemachineref (Variables|Default|GetDanceMachineRef))
  ;[0 0 0 0.5] This checks whether the dance note hitbox overlaps the component on the VRPawn's Hand "DanceHand". If it is the VR hand, the note is marked as resolved and prints a temporary hit mesage and stops movement on the timeline, then destroys itself. This helps prevent double counting
  (if (not (Variables|Default|GetHasBeenResolved))
    (if (Components|ComponentHasTag OtherComp "DanceHand")
      (Variables|Default|SetHasBeenResolved true)
      (Variables|/Script/Engine.PrimitiveComponent|SetbGenerateOverlapEvents (Variables|Default|GetNoteHitBox) false)
      (Development|PrintString "Hit Note" true true "(R=0.000000,G=0.660000,B=1.000000,A=1.000000)" 7.0)
      (Utilities|IsValid _dancemachineref
        (:Is%20Valid
          (Audio|Components|Audio|Stop (Variables|Default|GetTL_MoveNote))
          (Default|RegisterNoteHit _dancemachineref))
        (:Is%20Not%20Valid
          _))
      (Actor|DestroyActor))))

(event Custom|ApplyArrowMesh
  ;[0.8333 0.3342 0.4681 0.5] Checks the note’s ArrowDirection value and swaps the ArrowMesh component to the matching custom Blender arrow model.
  (switch Utilities|FlowControl|Switch|SwitchonE_DanceArrowType (Variables|Default|GetArrowDirection)
    (:NewEnumerator0
      (Components|StaticMesh|SetStaticMesh (Variables|Default|GetArrowMesh) (Variables|Default|GetDownArrowMesh)))
    (:NewEnumerator1
      (Components|StaticMesh|SetStaticMesh (Variables|Default|GetArrowMesh) (Variables|Default|GetUpArrowMesh)))
    (:NewEnumerator2
      (Components|StaticMesh|SetStaticMesh (Variables|Default|GetArrowMesh) (Variables|Default|GetLeftArrowMesh)))
    (:NewEnumerator3
      (Components|StaticMesh|SetStaticMesh (Variables|Default|GetArrowMesh) (Variables|Default|GetRightArrowMesh)))))

(event EventBeginPlay
  ;[0.1984 0.1724 1 0.4522] Runs when the dance note first appears. It saves the note’s starting position in StartLocation, then checks the ArrowDirection value to decide which way the note should move.
  (CallFunction|ApplyArrowMesh)
  (Variables|Default|SetStartLocation (Transformation|GetActorLocation))
  (switch Utilities|FlowControl|Switch|SwitchonE_DanceArrowType (Variables|Default|GetArrowDirection)
    (:NewEnumerator0
      ;[0.1371 0.06123 0.4479 0.5652] This works out where the notes go. It starts from the note’s current position, moves that position to the right by the MoveDistance amount, saves that new position as EndLocation, and then starts the Timeline so the note can begin moving.
      (Variables|Default|SetEndLocation (+ (* (Transformation|GetActorUpVector) (Variables|Default|GetMoveDistance)) (Variables|Default|GetStartLocation)))
      (Components|Timeline|PlayfromStart (Variables|Default|GetTL_MoveNote)))
    (:NewEnumerator1
      (Variables|Default|SetEndLocation (+ (* (Transformation|GetActorUpVector) (* (Variables|Default|GetMoveDistance) -1.0)) (Variables|Default|GetStartLocation)))
      (Components|Timeline|PlayfromStart (Variables|Default|GetTL_MoveNote)))
    (:NewEnumerator2
      (Variables|Default|SetEndLocation (+ (* (Transformation|GetActorRightVector) (* (Variables|Default|GetMoveDistance) -1.0)) (Variables|Default|GetStartLocation)))
      (Components|Timeline|PlayfromStart (Variables|Default|GetTL_MoveNote)))
    (:NewEnumerator3
      (Variables|Default|SetEndLocation (+ (* (Transformation|GetActorRightVector) (Variables|Default|GetMoveDistance)) (Variables|Default|GetStartLocation)))
      (Components|Timeline|PlayfromStart (Variables|Default|GetTL_MoveNote)))))

(fn ConstructionScript)