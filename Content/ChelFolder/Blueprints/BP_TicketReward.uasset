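; BP_TicketReward is a VR arcade prize ticket, hidden at BeginPlay until ActivateTicket reveals it after a dance machine win.
; A Timeline lerps it forward along its facing vector to simulate printing, then enables collision.
; Once printed, overlapping a DanceHand-tagged component attaches it to that hand for carrying.
; InsertIntoTicketMachine detaches it, disables collision, and slides it to the given insert point on a second Timeline before hiding it.
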(event OnComponentBeginOverlap(CollectBox)
  (params (OverlappedComponent :type Primitive%20Component%20Object%20Reference) (OtherActor :type Actor%20Object%20Reference) (OtherComp :type Primitive%20Component%20Object%20Reference) (OtherBodyIndex :type Integer) (bFromSweep :type Boolean) (SweepResult :type Hit%20Result%20Structure%20%28by%20ref%29))
  ;[0.06921 0.04655 0.15 0.5] When the printed ticket is touched by a VR hand, the ticket checks that it has finished printing and has not already been collected, then attaches itself to the hand so the player can carry it to the ticket machine.
  (if (Variables|Default|GetHasPrinted)
    (if (not (Variables|Default|GetIsCollected))
      (if (Components|ComponentHasTag OtherComp "DanceHand")
        (Variables|Default|SetIsCollected true)
        (Transformation|AttachComponentToComponent OtherComp "None" "KeepWorld" "KeepWorld" "KeepWorld" false)))))

(event Custom|ActivateTicket
  ;[0.2587 0.5052 0.3022 0.5] Moves the ticket from its saved start position to its calculated printed-out position while the Timeline plays, creating the effect of a ticket sliding out of the arcade machine.
  (Rendering|SetActorHiddenInGame false)
  (Collision|SetActorEnableCollision false)
  (Variables|Default|SetHasPrinted false)
  (bind _output_get (Variables|Default|SetPrintStartLocation (Transformation|GetActorLocation)))
  (Variables|Default|SetPrintEndLocation (+ _output_get (* (Transformation|GetActorForwardVector) (Variables|Default|GetPrintDistance))))
  (bind _alpha (Timeline|TL_PrintTicket PlayFromStart)
    (:Update
      (Transformation|SetActorLocation (Math|Vector|Lerp(Vector) (Variables|Default|GetPrintStartLocation) (Variables|Default|GetPrintEndLocation) _alpha) false false))
    (:Finished
      (Variables|Default|SetHasPrinted true)
      (Collision|SetActorEnableCollision true))))

(event Custom|ConsumeTicket
  ;[0.1332 0.15 0.09322 0.5] Consumes the collected ticket when it is inserted into the ticket machine. The ticket detaches from the hand, hides itself, and disables collision so it can no longer be used.
  (Transformation|DetachFromActor "KeepWorld" "KeepWorld" "KeepWorld")
  (Rendering|SetActorHiddenInGame false)
  (Collision|SetActorEnableCollision false))

(event Custom|InsertIntoTicketMachine
  (params (InsertPoint :type Scene%20Component%20Object%20Reference))
  ;[0.15 0.0593 0.02891 0.5] When the collected ticket reaches the ticket machine slot, it detaches from the hand, disables collision to prevent repeat overlaps, then uses a Timeline to slide into the insert point before hiding itself.
  (if (not (Variables|Default|GetIsBeingInserted))
    (Variables|Default|SetIsBeingInserted true)
    (Transformation|DetachFromActor "KeepWorld" "KeepWorld" "KeepWorld")
    (Collision|SetActorEnableCollision false)
    (Variables|Default|SetInsertStartLocation (Transformation|GetActorLocation))
    (Variables|Default|SetInsertEndLocation (Transformation|GetWorldLocation InsertPoint))
    (bind _alpha (Timeline|TL_InsertTicket PlayFromStart)
      (:Update
        (Transformation|SetActorLocation (Math|Vector|Lerp(Vector) (Variables|Default|GetInsertStartLocation) (Variables|Default|GetInsertEndLocation) _alpha) false false))
      (:Finished
        (Rendering|SetActorHiddenInGame true)
        (Collision|SetActorEnableCollision false)
        (Development|PrintString "Ticket Inserted" true true "(R=1.000000,G=0.185861,B=0.000000,A=1.000000)" 9.0)
        (Variables|Default|SetIsCollected false)))))

(event EventBeginPlay
  ;[0.15 0.07281 0.1287 0.5] Hides the ticket and disables collision when the level starts so the reward only appears after the player wins the dance machine round.
  (Rendering|SetActorHiddenInGame true)
  (Collision|SetActorEnableCollision false))

(event Collision|EventActorBeginOverlap
  (params (OtherActor :type Actor%20Object%20Reference)))

(event EventTick
  (params (DeltaSeconds :type Float%20%28single-precision%29)))

(fn ConstructionScript)