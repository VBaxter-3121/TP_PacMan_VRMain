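; Ticket machine that takes inserted BP_TicketReward actors and unlocks four mini prizes and a final code paper at ticket-count goals.
; The slot overlap starts insertion, and ConfirmTicketInserted increments the total and checks each one-time reward.
; Unlocks reveal the initially hidden reward, update the ticket widget's number and swing the cabinet flap open via a shared rotation-lerp Timeline.
; A mini prize leaving the cabinet box reverses that Timeline after a delay.
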(event OnComponentBeginOverlap(TickerInsertBox)
  (params (OverlappedComponent :type Primitive%20Component%20Object%20Reference) (OtherActor :type Actor%20Object%20Reference) (OtherComp :type Primitive%20Component%20Object%20Reference) (OtherBodyIndex :type Integer) (bFromSweep :type Boolean) (SweepResult :type Hit%20Result%20Structure%20%28by%20ref%29))
  ;[0.05304 0.09357 0.15 0.5] Checks whether the inserted object is a BP_TicketReward. If the player brings the collected ticket into the slot, the ticket machine consumes it and confirms the reward was accepted.
  (bind _asbp_ticket_reward (Utilities|Casting|CastToBP_TicketReward OtherActor))
  (Default|InsertIntoTicketMachine _asbp_ticket_reward (Variables|Default|GetTicketInsertPoint) self))

(event OnComponentEndOverlap(PrizeCabinetBox)
  (params (OverlappedComponent :type Primitive%20Component%20Object%20Reference) (OtherActor :type Actor%20Object%20Reference) (OtherComp :type Primitive%20Component%20Object%20Reference) (OtherBodyIndex :type Integer))
  ;[0.15 0.04844 0.04844 0.5] When the active mini prize leaves the cabinet area, the ticket machine knows the player has taken it and reverses the flap Timeline so the cabinet shuts again.
  (if (Math|Boolean|ORBoolean (== OtherActor (Variables|Default|GetMiniPrizeRef)) (== OtherActor (Variables|Default|GetMiniPrizeRef2)) (== OtherActor (Variables|Default|GetMiniPrizeRef3)) (== OtherActor (Variables|Default|GetMiniPrizeRef4)))
    (if (Variables|Default|GetPrizeIsInCabinet)
      (Variables|Default|SetPrizeIsInCabinet false)
      (Utilities|FlowControl|Delay 2.0)
      ;[0.0928 0.06734 0.15 0.5] Reveals the mini prize, saves the cabinet flap’s closed rotation, calculates its open rotation, then plays a Timeline so the door swings down smoothly.
      (bind _alpha (Timeline|TL_OpenCabinetDoor ReverseFromEnd)
        (:Update
          (Transformation|SetRelativeRotation (Variables|Default|GetCabinetDoorHinge) (Math|Rotator|Lerp(Rotator) (Variables|Default|GetDoorClosedRotation) (Variables|Default|GetDoorOpenRotation) _alpha) false false))))))

(event Custom|RevealMiniPrize
  ;[0.0928 0.06734 0.15 0.5] Reveals the mini prize, saves the cabinet flap’s closed rotation, calculates its open rotation, then plays a Timeline so the door swings down smoothly.
  (Variables|Default|SetHasGivenMiniPrize true)
  (Variables|Default|SetPrizeIsInCabinet true)
  (Utilities|IsValid (Variables|Default|GetMiniPrizeRef)
    (:Is%20Valid
      (Default|ActivateMiniPrize (Variables|Default|GetMiniPrizeRef))
      (bind _output_get (Variables|Default|SetDoorClosedRotation (Variables|/Script/Engine.SceneComponent|GetRelativeRotation (Variables|Default|GetCabinetDoorHinge))))
      (Variables|Default|SetDoorOpenRotation (Math|Rotator|CombineRotators _output_get (Math|Rotator|MakeRotator (Variables|Default|GetDoopOpenAngle) 0.0 0.0)))
      (bind _alpha (Timeline|TL_OpenCabinetDoor PlayFromStart)
        (:Update
          (Transformation|SetRelativeRotation (Variables|Default|GetCabinetDoorHinge) (Math|Rotator|Lerp(Rotator) (Variables|Default|GetDoorClosedRotation) (Variables|Default|GetDoorOpenRotation) _alpha) false false))))))

(event Custom|CheckCodeReward
  ;[0.02943 0.03562 0.15 0.5] Checks whether the ticket total has reached the final code reward amount. If the code has not already been given, the ticket machine reveals the hidden code paper reward
  (if (>= (Variables|Default|GetTicketsInserted) (Variables|Default|GetTicketsNeededForCode))
    (if (not (Variables|Default|GetHasGivenCode))
      (CallFunction|RevealCodePaperReward)
      (bind _aswbp_ticket (Utilities|Casting|CastToWBP_Ticket (UserInterface|GetWidget (Variables|Default|GetWidget))))
      (Default|SetNumber _aswbp_ticket "0"))))

(event Custom|CheckMiniPrizeReward
  ;[0.1009 0.15 0.05017 0.5] Checks whether the current ticket total has reached the mini prize goal. If the reward has not already been given, the ticket machine opens its cabinet and reveals the prize.
  (if (>= (Variables|Default|GetTicketsInserted) (Variables|Default|GetMiniPrizeTicketGoal))
    (if (not (Variables|Default|GetHasGivenMiniPrize))
      (CallFunction|RevealMiniPrize)
      (bind _aswbp_ticket (Utilities|Casting|CastToWBP_Ticket (UserInterface|GetWidget (Variables|Default|GetWidget))))
      (Default|SetNumber _aswbp_ticket "4"))))

(event Custom|CheckMiniPrizeReward3
  ;[0.1009 0.15 0.05017 0.5] Checks whether the current ticket total has reached the mini prize goal. If the reward has not already been given, the ticket machine opens its cabinet and reveals the prize.
  (if (>= (Variables|Default|GetTicketsInserted) (Variables|Default|GetMiniPrize3TicketGoal))
    (if (not (Variables|Default|GetHasGivenMiniPrize3))
      (CallFunction|RevealMiniPrize3)
      (bind _aswbp_ticket (Utilities|Casting|CastToWBP_Ticket (UserInterface|GetWidget (Variables|Default|GetWidget))))
      (Default|SetNumber _aswbp_ticket "2"))))

(event Custom|CheckMiniPrizeReward4
  ;[0.1009 0.15 0.05017 0.5] Checks whether the current ticket total has reached the mini prize goal. If the reward has not already been given, the ticket machine opens its cabinet and reveals the prize.
  (if (>= (Variables|Default|GetTicketsInserted) (Variables|Default|GetMiniPrize4TicketGoal))
    (if (not (Variables|Default|GetHasGivenMiniPrize4))
      (CallFunction|RevealMiniPrize4)
      (bind _aswbp_ticket (Utilities|Casting|CastToWBP_Ticket (UserInterface|GetWidget (Variables|Default|GetWidget))))
      (Default|SetNumber _aswbp_ticket "1"))))

(event Custom|ConfirmTicketInserted
  ;[0.09718 0.15 0.005707 0.5] Runs after a ticket has fully finished sliding into the machine. It adds one to the ticket total, then checks whether the mini prize or final code reward should unlock.
  (Variables|Default|SetTicketsInserted (+ (Variables|Default|GetTicketsInserted) 1))
  (CallFunction|CheckMiniPrizeReward)
  (CallFunction|CheckMiniPrize2Reward)
  (CallFunction|CheckMiniPrizeReward3)
  (CallFunction|CheckMiniPrizeReward4)
  (CallFunction|CheckCodeReward))

(event Custom|CheckMiniPrize2Reward
  ;[0.02793 0.15 0.08273 0.5] Checks whether the ticket total has reached the second mini prize goal. If this reward has not already been given, the machine reveals the second prize.
  (if (>= (Variables|Default|GetTicketsInserted) (Variables|Default|GetMiniPrize2TicketGoal))
    (if (not (Variables|Default|GetHasGivenMiniPrize2))
      (CallFunction|RevealMiniPrize2 self)
      (bind _aswbp_ticket (Utilities|Casting|CastToWBP_Ticket (UserInterface|GetWidget (Variables|Default|GetWidget))))
      (Default|SetNumber _aswbp_ticket "3"))))

(event Custom|RevealMiniPrize4
  (Variables|Default|SetHasGivenMiniPrize4 true)
  (Variables|Default|SetPrizeIsInCabinet true)
  (Utilities|IsValid (Variables|Default|GetMiniPrizeRef4)
    (:Is%20Valid
      (Default|ActivateMiniPrize (Variables|Default|GetMiniPrizeRef4))
      (bind _output_get (Variables|Default|SetDoorClosedRotation (Variables|/Script/Engine.SceneComponent|GetRelativeRotation (Variables|Default|GetCabinetDoorHinge))))
      (Variables|Default|SetDoorOpenRotation (Math|Rotator|CombineRotators _output_get (Math|Rotator|MakeRotator (Variables|Default|GetDoopOpenAngle) 0.0 0.0)))
      ;[0.0928 0.06734 0.15 0.5] Reveals the mini prize, saves the cabinet flap’s closed rotation, calculates its open rotation, then plays a Timeline so the door swings down smoothly.
      (bind _alpha (Timeline|TL_OpenCabinetDoor PlayFromStart)
        (:Update
          (Transformation|SetRelativeRotation (Variables|Default|GetCabinetDoorHinge) (Math|Rotator|Lerp(Rotator) (Variables|Default|GetDoorClosedRotation) (Variables|Default|GetDoorOpenRotation) _alpha) false false))))))

(event Custom|RevealCodePaperReward
  ;[0.0572 0.02566 0.15 0.5] Reveals the final code paper reward and opens the cabinet flap when the player has inserted enough tickets to complete the ticket machine reward chain.
  (Variables|Default|SetHasGivenCode true)
  (Variables|Default|SetPrizeIsInCabinet true)
  (Rendering|SetVisibility (Variables|Default|GetCodePaperMesh) true false)
  (bind _output_get (Variables|Default|SetDoorClosedRotation (Variables|/Script/Engine.SceneComponent|GetRelativeRotation (Variables|Default|GetCabinetDoorHinge))))
  (Variables|Default|SetDoorOpenRotation (Math|Rotator|CombineRotators _output_get (Math|Rotator|MakeRotator (Variables|Default|GetDoopOpenAngle) 0.0 0.0)))
  ;[0.0928 0.06734 0.15 0.5] Reveals the mini prize, saves the cabinet flap’s closed rotation, calculates its open rotation, then plays a Timeline so the door swings down smoothly.
  (bind _alpha (Timeline|TL_OpenCabinetDoor PlayFromStart)
    (:Update
      (Transformation|SetRelativeRotation (Variables|Default|GetCabinetDoorHinge) (Math|Rotator|Lerp(Rotator) (Variables|Default|GetDoorClosedRotation) (Variables|Default|GetDoorOpenRotation) _alpha) false false))))

(event Custom|RevealMiniPrize2
  ;[0.0382 0.02732 0.06125] Activates the second grabbable prize and reopens the cabinet flap when the second ticket reward threshold is reached.
  (Variables|Default|SetHasGivenMiniPrize2 true)
  (Variables|Default|SetPrizeIsInCabinet true)
  (Utilities|IsValid (Variables|Default|GetMiniPrizeRef2)
    (:Is%20Valid
      (Default|ActivateMiniPrize (Variables|Default|GetMiniPrizeRef2))
      (bind _output_get (Variables|Default|SetDoorClosedRotation (Variables|/Script/Engine.SceneComponent|GetRelativeRotation (Variables|Default|GetCabinetDoorHinge))))
      (Variables|Default|SetDoorOpenRotation (Math|Rotator|CombineRotators _output_get (Math|Rotator|MakeRotator (Variables|Default|GetDoopOpenAngle) 0.0 0.0)))
      ;[0.0928 0.06734 0.15 0.5] Reveals the mini prize, saves the cabinet flap’s closed rotation, calculates its open rotation, then plays a Timeline so the door swings down smoothly.
      (bind _alpha (Timeline|TL_OpenCabinetDoor PlayFromStart)
        (:Update
          (Transformation|SetRelativeRotation (Variables|Default|GetCabinetDoorHinge) (Math|Rotator|Lerp(Rotator) (Variables|Default|GetDoorClosedRotation) (Variables|Default|GetDoorOpenRotation) _alpha) false false))))))

(event Custom|RevealMiniPrize3
  (Variables|Default|SetHasGivenMiniPrize3 true)
  (Variables|Default|SetPrizeIsInCabinet true)
  (Utilities|IsValid (Variables|Default|GetMiniPrizeRef3)
    (:Is%20Valid
      (Default|ActivateMiniPrize (Variables|Default|GetMiniPrizeRef3))
      (bind _output_get (Variables|Default|SetDoorClosedRotation (Variables|/Script/Engine.SceneComponent|GetRelativeRotation (Variables|Default|GetCabinetDoorHinge))))
      (Variables|Default|SetDoorOpenRotation (Math|Rotator|CombineRotators _output_get (Math|Rotator|MakeRotator (Variables|Default|GetDoopOpenAngle) 0.0 0.0)))
      ;[0.0928 0.06734 0.15 0.5] Reveals the mini prize, saves the cabinet flap’s closed rotation, calculates its open rotation, then plays a Timeline so the door swings down smoothly.
      (bind _alpha (Timeline|TL_OpenCabinetDoor PlayFromStart)
        (:Update
          (Transformation|SetRelativeRotation (Variables|Default|GetCabinetDoorHinge) (Math|Rotator|Lerp(Rotator) (Variables|Default|GetDoorClosedRotation) (Variables|Default|GetDoorOpenRotation) _alpha) false false))))))

(event EventBeginPlay
  (bind _miniprizeref3 (Variables|Default|GetMiniPrizeRef3))
  (bind _miniprizeref4 (Variables|Default|GetMiniPrizeRef4))
  ;[0.02207 0.15 0.13 0.5] Hides and disables the grabbable prize rewards at level start so they only become available once the ticket machine unlocks them.
  (Utilities|IsValid (Variables|Default|GetMiniPrizeRef)
    (:Is%20Valid
      (Default|DeactivateMiniPrize (Variables|Default|GetMiniPrizeRef))
      (Utilities|IsValid (Variables|Default|GetMiniPrizeRef2)
        (:Is%20Valid
          (Default|DeactivateMiniPrize (Variables|Default|GetMiniPrizeRef2))
          (Utilities|IsValid _miniprizeref3
            (:Is%20Valid
              (Default|DeactivateMiniPrize _miniprizeref3)
              (Utilities|IsValid _miniprizeref4
                (:Is%20Valid
                  (Default|DeactivateMiniPrize _miniprizeref4)
                  (Rendering|SetVisibility (Variables|Default|GetCodePaperMesh) false false))))))))))

(fn ConstructionScript)