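; BP_DanceMachine is an interactable dance machine for the VR pawn, currently a placeholder that only toggles state and prints debug messages.
; InteractBox overlaps register the machine on VRPawn_chels and show or hide PromptWidget based on proximity.
; StartDanceMachine runs only when the player is near and the machine is idle.
; A temporary test delay then calls StopDanceMachine, which restores the prompt if the player is still inside.
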(event OnComponentBeginOverlap(InteractBox)
  (params (OverlappedComponent :type Primitive%20Component%20Object%20Reference) (OtherActor :type Actor%20Object%20Reference) (OtherComp :type Primitive%20Component%20Object%20Reference) (OtherBodyIndex :type Integer) (bFromSweep :type Boolean) (SweepResult :type Hit%20Result%20Structure%20%28by%20ref%29))
  ;[0.1527 0.2539 0.924 0.5] When the Player enters the InteractBox, store the player and allow the machine to start.
  ; The prompt appears because the player is now close enough to interact.
  (bind _asvrpawn_chels (Utilities|Casting|CastToVRPawn_chels OtherActor))
  (Variables|Default|SetCurrentPawn _asvrpawn_chels)
  (Variables|/Game/ChelFolder/VRPawn_chels.VRPawn_chels_C|SetCurrentDanceMachine _asvrpawn_chels self)
  (Variables|Default|SetCanStartMachine true)
  (Rendering|SetVisibility (Variables|Default|GetPromptWidget) true false))

(event OnComponentEndOverlap(InteractBox)
  (params (OverlappedComponent :type Primitive%20Component%20Object%20Reference) (OtherActor :type Actor%20Object%20Reference) (OtherComp :type Primitive%20Component%20Object%20Reference) (OtherBodyIndex :type Integer))
  ;[0.2836 0.9073 0.2859 0.5] When the Player  leaves the InteractBox, clear the player and stop the machine from starting.
  ; The prompt hides so the machine cannot be used from too far away.
  (bind _asvrpawn_chels (Utilities|Casting|CastToVRPawn_chels OtherActor))
  (Variables|Default|SetCurrentPawn 0)
  (Variables|/Game/ChelFolder/VRPawn_chels.VRPawn_chels_C|SetCurrentDanceMachine _asvrpawn_chels 0)
  (Variables|Default|SetCanStartMachine false)
  (Rendering|SetVisibility (Variables|Default|GetPromptWidget) false false))

(event Custom|StartDanceMachine
  ;[0.15 0.039 0.07553 0.5] Check if the machine is already playing before running the start logic.
  ; If IsPlaying is true, block another start and show debug feedback instead.
  (if (Variables|Default|GetIsPlaying)
    (Development|PrintString "Machine already playing")
    (else
      ;[0.8323 0.1158 0.1368 0.5] StartDanceMachine checks if the player is close enough before starting.
      ; If CanStartMachine is true, the machine starts and hides the prompt.
      (if (Variables|Default|GetCanStartMachine)
        (Variables|Default|SetIsPlaying true)
        (Development|PrintString "Dance Machine Started")
        (Rendering|SetVisibility (Variables|Default|GetPromptWidget) false false)
        ;[0.15 0.05078 0.05585 0.5] Temporary test delay: keep the machine active for 3 seconds, then call StopDanceMachine to return it to an idle state.
        (Utilities|FlowControl|Delay 3.0)
        (CallFunction|StopDanceMachine)
        (else
          (Development|PrintString "Too far from machine"))))))

(event Custom|StopDanceMachine
  ;[0.5938 0.07165 0.1649 0.5] StopDanceMachine sets IsPlaying back to false, then checks CanStartMachine.
  ; If the player is still near, show the PromptWidget again. If not, keep it hidden.
  (Variables|Default|SetIsPlaying false)
  (if (Variables|Default|GetCanStartMachine)
    (Rendering|SetVisibility (Variables|Default|GetPromptWidget) true false)
    (else
      (Rendering|SetVisibility (Variables|Default|GetPromptWidget) false false))))

(event EventBeginPlay
  ;[0.3373 0.7939 0.9906 0.5] On BeginPlay, hide the machine prompt so it does not aappear as soon as the level starts.
  (Rendering|SetVisibility (Variables|Default|GetPromptWidget) false false))

(fn ConstructionScript)