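; BP_MiniPrize is a cabinet prize actor that stays locked away until it is unlocked and can then be picked up in VR.
; DeactivateMiniPrize hides it, turns off collision and stops physics on its static mesh, so it cannot fall or be grabbed early.
; ActivateMiniPrize reverses all three so the existing VR grab system can take it.
; Both events are triggered externally, as BeginPlay, overlap and Tick are disabled stubs.
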(event Custom|DeactivateMiniPrize
  ;[0.15 0.15 0.15 0.5] Hides and freezes the prize before it is unlocked so it stays inside the cabinet, cannot be grabbed early, and does not fall due to physics.
  (Rendering|SetActorHiddenInGame true)
  (Collision|SetActorEnableCollision false)
  (Physics|SetSimulatePhysics (Variables|Default|GetStaticMesh) false))

(event Custom|ActivateMiniPrize
  ;[0.15 0.15 0.15 0.5] Reveals the unlocked prize, restores collision, and re-enables physics so the existing VR grabbable system can pick it up.
  (Rendering|SetActorHiddenInGame false)
  (Collision|SetActorEnableCollision true)
  (Physics|SetSimulatePhysics (Variables|Default|GetStaticMesh) true))

(event EventBeginPlay
  (|CallParentFunction) ; This node is disabled and will not be called.\nDrag off pins to build functionality.
)

(event Collision|EventActorBeginOverlap
  (params (OtherActor :type Actor%20Object%20Reference))
  (|CallParentFunction OtherActor) ; This node is disabled and will not be called.\nDrag off pins to build functionality.
)

(event EventTick
  (params (DeltaSeconds :type Float%20%28single-precision%29))
  (|CallParentFunction DeltaSeconds) ; This node is disabled and will not be called.\nDrag off pins to build functionality.
)

(fn ConstructionScript
  (|CallParentFunction))