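; Behavior tree task that carries out Pac-Man's attack on the VR player by moving both to a death location.
; On execute it reads the death location from Pac-Man's test controller and disables gravity on both pawns' capsules.
; It teleports Pac-Man to that spot and the player to a small X offset from it.
; The task then finishes as failed; a failed cast stops it without finishing.
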(event EventReceiveExecute
  (params (OwnerActor :type Actor%20Object%20Reference))
  (bind _asbp_pac__man (Utilities|Casting|CastToBP_Pac-Man OwnerActor))
  (bind _output_get (Variables|Default|SetPacMan _asbp_pac__man))
  (bind _asbp_pac_man_test_controller (Utilities|Casting|CastToBP_PacMan_Test_Controller (Pawn|GetController _output_get)))
  (Variables|Default|SetDeath%20Location (Variables|/Game/VincentFolder/Blueprints/Pacman/BP_PacMan_Test_Controller.BP_PacMan_Test_Controller_C|GetDeathLocation _asbp_pac_man_test_controller))
  (bind _asvrpawn (Utilities|Casting|CastToVRPawn (Game|Player|GetPlayerPawn 0)))
  (bind _output_get_2 (Variables|Default|SetPlayer _asvrpawn))
  (Physics|SetEnableGravity (Variables|/Script/Engine.Character|GetCapsuleComponent _output_get_2) false)
  (Physics|SetEnableGravity (Variables|/Script/Engine.Character|GetCapsuleComponent (Variables|Default|GetPacMan)) false)
  (Transformation|SetActorTransform (Variables|Default|GetPacMan) (Math|Transform|MakeTransform (Variables|Default|GetDeath%20Location) "0, 0, 0" (Transformation|GetActorScale3D (Variables|Default|GetPacMan))))
  (Transformation|SetActorTransform (Variables|Default|GetPlayer) (Math|Transform|MakeTransform (+ (Variables|Default|GetDeath%20Location) "100.000000,0.000000,0.000000") "0, 0, 0" "1.000000,1.000000,1.000000"))
  (AI|BehaviorTree|FinishExecute false))