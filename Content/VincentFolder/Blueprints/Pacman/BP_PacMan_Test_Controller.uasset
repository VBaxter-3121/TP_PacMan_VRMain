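; AI controller for a test Pac-Man character that tracks the player by sight and hearing.
; It starts the BT_PacMan_Test behavior tree, then routes AI Perception updates by sense to update the blackboard.
; Sight sets the player target, or records the last seen location when contact is lost.
; Hearing flags noises and stores their location as the target, without resetting the flag here.
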(event OnTargetPerceptionUpdated(AIPerception)
  (params (Actor :type Actor%20Object%20Reference) (Stimulus :type AI%20Stimulus%20Structure))
  ;[0.15 0.15 0.15 0.5] Update blackboard keys based on perception data
  (Variables|Default|SetSensedActor Actor)
  (bind _output_get (Variables|Default|SetStimulus Stimulus))
  (bind _returnvalue (Class|AIPerceptionSystem|GetSenseClassforStimulus _output_get))
  (switch string (Utilities|GetClassDisplayName _returnvalue)
    (:AISense_Sight
      (CallFunction|SightUpdated))
    (:AISense_Hearing
      (CallFunction|HearingUpdated))))

(event EventBeginPlay
  ;[0.15 0.15 0.15 0.5] Initialise AI and relevant variables
  (AI|RunBehaviorTree "/Game/VincentFolder/Blueprints/Pacman/BT_PacMan_Test.BT_PacMan_Test")
  (Variables|Default|SetPacmanBlackboard (AI|GetBlackboard 0)))

(fn ConstructionScript)

(fn SightUpdated
  (if (.bsuccessfullysensed (Variables|Default|GetStimulus)) ; True if player sighted, False if lost sight of player
    ;[0.15 0.15 0.15 0.5] Player in sight
    (AI|Components|Blackboard|SetValueasBool (Variables|Default|GetPacmanBlackboard) (Variables|Default|GetPlayerSeen) true)
    (AI|Components|Blackboard|SetValueasObject (Variables|Default|GetPacmanBlackboard) (Variables|Default|GetPlayer) (Variables|Default|GetSensedActor))
    (AI|Components|Blackboard|ClearValue (Variables|Default|GetPacmanBlackboard) (Variables|Default|GetTargetLocation))
    (AI|Components|Blackboard|ClearValue (Variables|Default|GetPacmanBlackboard) (Variables|Default|GetLastSeenLocation))
    (else
      ;[0.15 0.15 0.15 0.5] Lost sight of player
      (AI|Components|Blackboard|SetValueasBool (Variables|Default|GetPacmanBlackboard) (Variables|Default|GetPlayerSeen) false)
      (AI|Components|Blackboard|ClearValue (Variables|Default|GetPacmanBlackboard) (Variables|Default|GetPlayer))
      (AI|Components|Blackboard|SetValueasVector (Variables|Default|GetPacmanBlackboard) (Variables|Default|GetLastSeenLocation) (.stimuluslocation (Variables|Default|GetStimulus))))))

(fn HearingUpdated
  (if (.bsuccessfullysensed (Variables|Default|GetStimulus))
    ;[0.15 0.15 0.15 0.5] Noise heard
    (AI|Components|Blackboard|SetValueasBool (Variables|Default|GetPacmanBlackboard) (Variables|Default|GetNoiseHeard) true)
    (AI|Components|Blackboard|SetValueasVector (Variables|Default|GetPacmanBlackboard) (Variables|Default|GetTargetLocation) (.stimuluslocation (Variables|Default|GetStimulus)))
    (AI|Components|Blackboard|ClearValue (Variables|Default|GetPacmanBlackboard) (Variables|Default|GetLastSeenLocation))))