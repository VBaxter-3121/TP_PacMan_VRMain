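; VR air hockey table actor that runs a scored match between the player and an enemy bat.
; A trigger sphere registers the table with the VRPawn and allows starting a game; StartGame resets scores, respawns the puck and moves the bat.
; Goal overlaps respawn the puck and update the opposing score widget.
; While the puck overlaps PushBoundary, Tick applies negative-Y force to it; EndGame is empty.
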(event OnComponentBeginOverlap(PushBoundary)
  (params (OverlappedComponent :type Primitive%20Component%20Object%20Reference) (OtherActor :type Actor%20Object%20Reference) (OtherComp :type Primitive%20Component%20Object%20Reference) (OtherBodyIndex :type Integer) (bFromSweep :type Boolean) (SweepResult :type Hit%20Result%20Structure%20%28by%20ref%29))
  (Utilities|Casting|CastToBP_AirHockeyPuck OtherActor)
  (Variables|Default|SetPushPuck true)
  (Variables|Default|SetYDir -1.0))

(event OnComponentEndOverlap(PushBoundary)
  (params (OverlappedComponent :type Primitive%20Component%20Object%20Reference) (OtherActor :type Actor%20Object%20Reference) (OtherComp :type Primitive%20Component%20Object%20Reference) (OtherBodyIndex :type Integer))
  (Utilities|Casting|CastToBP_AirHockeyPuck OtherActor)
  (Variables|Default|SetPushPuck false))

(event OnComponentBeginOverlap(Goal1)
  (params (OverlappedComponent :type Primitive%20Component%20Object%20Reference) (OtherActor :type Actor%20Object%20Reference) (OtherComp :type Primitive%20Component%20Object%20Reference) (OtherBodyIndex :type Integer) (bFromSweep :type Boolean) (SweepResult :type Hit%20Result%20Structure%20%28by%20ref%29))
  (bind _asbp_air_hockey_puck (Utilities|Casting|CastToBP_AirHockeyPuck OtherActor))
  (Default|Respawn _asbp_air_hockey_puck)
  (Math|Integer|IncrementInt (Variables|Default|GetScore2)
    (:%20%20
      (bind _aswbp_air_hockey_score (Utilities|Casting|CastToWBP_AirHockeyScore (UserInterface|GetWidget (Variables|Default|GetScoreWidget2))))
      (Default|SetScore _aswbp_air_hockey_score (Variables|Default|GetScore2)))))

(event OnComponentBeginOverlap(Goal2)
  (params (OverlappedComponent :type Primitive%20Component%20Object%20Reference) (OtherActor :type Actor%20Object%20Reference) (OtherComp :type Primitive%20Component%20Object%20Reference) (OtherBodyIndex :type Integer) (bFromSweep :type Boolean) (SweepResult :type Hit%20Result%20Structure%20%28by%20ref%29))
  (bind _asbp_air_hockey_puck (Utilities|Casting|CastToBP_AirHockeyPuck OtherActor))
  (Default|Respawn _asbp_air_hockey_puck)
  (Math|Integer|IncrementInt (Variables|Default|GetScore1)
    (:%20%20
      (bind _aswbp_air_hockey_score (Utilities|Casting|CastToWBP_AirHockeyScore (UserInterface|GetWidget (Variables|Default|GetScoreWidget1))))
      (Default|SetScore _aswbp_air_hockey_score (Variables|Default|GetScore1)))))

(event OnComponentBeginOverlap(Sphere)
  (params (OverlappedComponent :type Primitive%20Component%20Object%20Reference) (OtherActor :type Actor%20Object%20Reference) (OtherComp :type Primitive%20Component%20Object%20Reference) (OtherBodyIndex :type Integer) (bFromSweep :type Boolean) (SweepResult :type Hit%20Result%20Structure%20%28by%20ref%29))
  (bind _asvrpawn (Utilities|Casting|CastToVRPawn OtherActor))
  (Variables|/Game/VRTemplate/Blueprints/VRPawn.VRPawn_C|SetCanStartGame _asvrpawn true)
  (Variables|/Game/VRTemplate/Blueprints/VRPawn.VRPawn_C|SetHockey _asvrpawn self))

(event OnComponentEndOverlap(Sphere)
  (params (OverlappedComponent :type Primitive%20Component%20Object%20Reference) (OtherActor :type Actor%20Object%20Reference) (OtherComp :type Primitive%20Component%20Object%20Reference) (OtherBodyIndex :type Integer))
  (bind _asvrpawn (Utilities|Casting|CastToVRPawn OtherActor))
  (Variables|/Game/VRTemplate/Blueprints/VRPawn.VRPawn_C|SetCanStartGame _asvrpawn false)
  (Variables|/Game/VRTemplate/Blueprints/VRPawn.VRPawn_C|SetHockey _asvrpawn 0))

(event Custom|StartGame
  (Variables|Default|SetScore1 0)
  (Variables|Default|SetScore2 0)
  (Default|Respawn (Variables|Default|GetPuck))
  (bind _aswbp_air_hockey_score (Utilities|Casting|CastToWBP_AirHockeyScore (UserInterface|GetWidget (Variables|Default|GetScoreWidget1))))
  (Default|SetScore _aswbp_air_hockey_score (Variables|Default|GetScore1))
  (bind _aswbp_air_hockey_score_2 (Utilities|Casting|CastToWBP_AirHockeyScore (UserInterface|GetWidget (Variables|Default|GetScoreWidget2))))
  (Default|SetScore _aswbp_air_hockey_score_2 (Variables|Default|GetScore2))
  (Default|Move (Variables|Default|GetEnemyBat)))

(event Custom|EndGame)

(event EventBeginPlay)

(event Collision|EventActorBeginOverlap
  (params (OtherActor :type Actor%20Object%20Reference)))

(event EventTick
  (params (DeltaSeconds :type Float%20%28single-precision%29))
  (if (Variables|Default|GetPushPuck)
    (Physics|AddForce (Variables|/Game/VincentFolder/Blueprints/Air_Hockey/BP_AirHockeyPuck.BP_AirHockeyPuck_C|GetStaticMesh (Variables|Default|GetPuck)) (Math|Vector|MakeVector 0.0 (* (Variables|Default|GetPushForce) (Variables|Default|GetYDir)) 0.0) "None" false)))

(fn ConstructionScript)