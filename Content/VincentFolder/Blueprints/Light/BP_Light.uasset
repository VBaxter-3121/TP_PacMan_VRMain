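; Point light actor with Constant, Flicker and Faulty passive effects chosen by LightEffect, plus a pursuit effect.
; Self-repeating timelines scale the starting intensity, with random delays for Flicker and Faulty and a random start time for Pursuit.
; Flicker and Faulty loops sit behind hardcoded false conditions, so never run.
; Pursuit repeats while IsPursued, then restores passive behaviour; SetIsPursued only sets the flag, without starting it.
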(event Custom|Flicker
  (if (not true)
    (Utilities|FlowControl|Delay (Math|Random|RandomFloatinRange (Variables|Default|GetFlickerLowerRange) (Variables|Default|GetFlickerUpperRange)))
    (bind _alpha (Timeline|FlickerTimeline PlayFromStart)
      (:Update
        (Rendering|Components|Light|SetIntensity (Variables|Default|GetPointLight) (* _alpha (Variables|Default|GetIntensity))))
      (:Finished
        (CallFunction|Flicker)))))

(event Custom|Faulty
  (if (not true)
    (Utilities|FlowControl|Delay (Math|Random|RandomFloatinRange (Variables|Default|GetFaultyLowerRange) (Variables|Default|GetFaultyUpperRange)))
    (bind _alpha (Timeline|FaultyTimeline PlayFromStart)
      (:Update
        (Rendering|Components|Light|SetIntensity (Variables|Default|GetPointLight) (* _alpha (Variables|Default|GetIntensity))))
      (:Finished
        (CallFunction|Faulty)))))

(event Custom|Pursuit
  (if (Variables|Default|GetIsPursued)
    (Utilities|FlowControl|Sequence
      (:then_0
        (bind _alpha (Timeline|PursuitTimeline SetNewTime)
          (:Update
            (Rendering|Components|Light|SetIntensity (Variables|Default|GetPointLight) (* _alpha (Variables|Default|GetIntensity))))
          (:Finished
            (CallFunction|Pursuit))))
      (:then_1
        (Timeline|PursuitTimeline Play)))
    (else
      (CallFunction|SetPassiveBehaviour))))

(event Custom|Constant
  (Rendering|Components|Light|SetIntensity (Variables|Default|GetPointLight) (* (Variables|Default|GetIntensity) 1.0)))

(event Custom|SetPassiveBehaviour
  (switch Utilities|FlowControl|Switch|SwitchonE_LightEffects (Variables|Default|GetLightEffect)
    (:NewEnumerator0
      (CallFunction|Constant))
    (:NewEnumerator1
      (CallFunction|Flicker))
    (:NewEnumerator2
      (Rendering|Components|Light|SetIntensity (Variables|Default|GetPointLight) (* (Variables|Default|GetIntensity) 0.1))
      (CallFunction|Faulty))))

(event Custom|SetIsPursued
  (params (IsPursued :type Boolean))
  (Variables|Default|SetIsPursued IsPursued))

(event EventBeginPlay
  (Variables|Default|SetIntensity (Variables|/Script/Engine.LightComponentBase|GetIntensity (Variables|Default|GetPointLight)))
  (CallFunction|SetPassiveBehaviour))

(event Collision|EventActorBeginOverlap
  (params (OtherActor :type Actor%20Object%20Reference)))

(event EventTick
  (params (DeltaSeconds :type Float%20%28single-precision%29)))

(fn ConstructionScript)