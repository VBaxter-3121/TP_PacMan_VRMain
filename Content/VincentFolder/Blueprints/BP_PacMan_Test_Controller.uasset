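; Test AI controller for a Pac-Man character that steers it toward a seen VR player or a heard noise.
; Runs BT_PacMan_Test on BeginPlay and handles AI perception updates.
; A successfully sensed VRPawn sight writes its stimulus location to the Blackboard destination key.
; Otherwise, any hearing stimulus writes to the same key, without checking the actor or sensing success.
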(event OnTargetPerceptionUpdated(AIPerception)
  (params (Actor :type Actor%20Object%20Reference) (Stimulus :type AI%20Stimulus%20Structure))
  (Variables|Default|SetActor Actor)
  (Variables|Default|SetStimulus Stimulus)
  (bind _playersighted (CallFunction|SightBehaviour))
  (if (not _playersighted)
    (CallFunction|SoundBehaviour)))

(event EventBeginPlay
  (AI|RunBehaviorTree "/Game/VincentFolder/Blueprints/BT_PacMan_Test.BT_PacMan_Test"))

(event EventTick
  (params (DeltaSeconds :type Float%20%28single-precision%29)))

(fn ConstructionScript)

(fn SightBehaviour
  (bind _stimulus (Variables|Default|GetStimulus))
  (bind _returnvalue (Class|AIPerceptionSystem|GetSenseClassforStimulus (Variables|Default|GetStimulus)))
  (if (== _returnvalue "/Script/AIModule.AISense_Sight")
    (Utilities|Casting|CastToVRPawn (Variables|Default|GetActor)
      (:then
        (if (.bsuccessfullysensed _stimulus)
          (AI|Components|Blackboard|SetValueasVector (AI|GetBlackboard 0) (Variables|Default|GetDestinationKey) (.stimuluslocation _stimulus))
          (return true)
          (else
            _)))
      (:CastFailed
        _)))
  (return false))

(fn SoundBehaviour
  (bind _returnvalue (Class|AIPerceptionSystem|GetSenseClassforStimulus (Variables|Default|GetStimulus)))
  (if (== _returnvalue "/Script/AIModule.AISense_Hearing")
    (AI|Components|Blackboard|SetValueasVector (AI|GetBlackboard 0) (Variables|Default|GetDestinationKey) (.stimuluslocation (Variables|Default|GetStimulus)))))