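; BP_ShutterButton is a powered door switch that lowers a referenced shutter door when something overlaps its box.
; Separate events toggle the power flag, and an overlap without power only prints a debug message.
; A powered overlap runs a timeline that slides the button mesh along its local Y and calls ShutterGoesDown on the door every update.
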(event OnComponentBeginOverlap(Box)
  (params (OverlappedComponent :type Primitive%20Component%20Object%20Reference) (OtherActor :type Actor%20Object%20Reference) (OtherComp :type Primitive%20Component%20Object%20Reference) (OtherBodyIndex :type Integer) (bFromSweep :type Boolean) (SweepResult :type Hit%20Result%20Structure%20%28by%20ref%29))
  (if (Variables|Default|GetIsPowerOn)
    (CallFunction|ButtonPressed)
    (else
      (Development|PrintString "Power off"))))

(event Custom|Button%20Pressed
  (bind _sm_doorswitchbutton (Variables|Default|GetSM_DoorSwitchButton))
  (bind _relativelocation (Variables|/Script/Engine.SceneComponent|GetRelativeLocation _sm_doorswitchbutton))
  (Variables|Default|SetIsPowerOn true)
  (bind _button_pressed (Timeline|ButtonPressed Play)
    (:Update
      (Transformation|SetRelativeLocation _sm_doorswitchbutton (Math|Vector|MakeVector (.x _relativelocation) _button_pressed (.z _relativelocation)) false false)
      (Default|ShutterGoesDown (Variables|Default|GetShutterDoorRef)))))

(event Custom|Power%20for%20button%20On
  (Variables|Default|SetIsPowerOn true))

(event Custom|Power%20for%20Button%20Off
  (Variables|Default|SetIsPowerOn false))

(event EventBeginPlay
  (if (Variables|Default|GetIsPowerOn)
    _))

(event Collision|EventActorBeginOverlap
  (params (OtherActor :type Actor%20Object%20Reference)))

(event EventTick
  (params (DeltaSeconds :type Float%20%28single-precision%29)))

(fn ConstructionScript)