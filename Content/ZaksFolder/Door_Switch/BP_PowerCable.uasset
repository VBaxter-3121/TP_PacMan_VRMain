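; BP_PowerCable is a power cable actor that drives the power state of a linked shutter button.
; On BeginPlay it activates its Niagara effect and, after a fixed delay, tells the referenced button that power is on.
; Its PowerisOn event switches the button's power off when IsPowerOn is false, and otherwise only sets the already-true flag again.
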(event Custom|Power%20is%20On
  (if (Variables|Default|GetIs%20Power%20On)
    (Variables|Default|SetIs%20Power%20On true)
    (else
      (Default|PowerforButtonOff (Variables|Default|GetShutterButtonRef)))))

(event EventBeginPlay
  (Components|Activation|Activate (Variables|Default|GetNiagara) false)
  (Utilities|FlowControl|Delay 13.7)
  (Default|PowerforButtonon (Variables|Default|GetShutterButtonRef)))

(event Collision|EventActorBeginOverlap
  (params (OtherActor :type Actor%20Object%20Reference)))

(event EventTick
  (params (DeltaSeconds :type Float%20%28single-precision%29)))

(fn ConstructionScript)