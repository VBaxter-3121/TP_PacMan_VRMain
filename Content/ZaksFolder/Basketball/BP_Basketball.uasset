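; BP_Basketball is a physics basketball actor that plays a bounce sound when it hits something.
; Component hits above a normal impulse threshold play the sound at the ball's location, with volume scaled by impact strength, slightly randomized pitch and distance attenuation.
; Playback starts partway into the sound asset.
; The hit handler's zero impulse and the BeginPlay HasScored self-assignment change nothing, and an unused velocity-based sound check remains disconnected.
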(event OnComponentHit(Basketball)
  (params (HitComponent :type Primitive%20Component%20Object%20Reference) (OtherActor :type Actor%20Object%20Reference) (OtherComp :type Primitive%20Component%20Object%20Reference) (NormalImpulse :type Vector :default "0, 0, 0") (Hit :type Hit%20Result%20Structure%20%28by%20ref%29))
  (bind _returnvalue (Math|Vector|VectorLength NormalImpulse))
  (Physics|AddImpulse (Variables|Default|GetBasketball) "0, 0, 0" "None" false)
  (if (>= _returnvalue 5e+01)
    (Audio|PlaySoundatLocation "/Game/ZaksFolder/Basketball/Basketball_Sound.Basketball_Sound" (Transformation|GetActorLocation) "0, 0, 0" (Math|Float|MapRangeClamped _returnvalue 2e+03 1.2e+04 0.4 1.0) (Math|Random|RandomFloatinRange 0.95 1.05) 3.1 "/Game/ZaksFolder/Basketball/SA_Basketball.SA_Basketball" 0 0 0)))

(event EventBeginPlay
  (Variables|Default|SetHasScored (Variables|Default|GetHasScored)))

(event Collision|EventActorBeginOverlap
  (params (OtherActor :type Actor%20Object%20Reference)))

(event EventTick
  (params (DeltaSeconds :type Float%20%28single-precision%29)))

(fn ConstructionScript)