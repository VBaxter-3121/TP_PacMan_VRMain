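; BP_BasketballMachine is a basketball machine actor that counts baskets toward a win score.
; Each BP_Basketball overlapping BasketCollision increments Score and updates a WBP_AirHockeyScore shown through the ScoreWidget component.
; At WinScore it calls Win, a placeholder that only prints a ticket message, then zeroes the displayed score without resetting Score itself.
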(event OnComponentBeginOverlap(BasketCollision)
  (params (OverlappedComponent :type Primitive%20Component%20Object%20Reference) (OtherActor :type Actor%20Object%20Reference) (OtherComp :type Primitive%20Component%20Object%20Reference) (OtherBodyIndex :type Integer) (bFromSweep :type Boolean) (SweepResult :type Hit%20Result%20Structure%20%28by%20ref%29))
  (bind _score (Variables|Default|GetScore))
  (Utilities|Casting|CastToBP_Basketball OtherActor)
  (Math|Integer|IncrementInt (Variables|Default|GetScore)
    (:%20%20
      (bind _aswbp_air_hockey_score (Utilities|Casting|CastToWBP_AirHockeyScore (UserInterface|GetWidget (Variables|Default|GetScoreWidget))))
      (Default|SetScore _aswbp_air_hockey_score _score)
      (if (>= _score (Variables|Default|GetWinScore))
        (CallFunction|Win)
        (Default|SetScore _aswbp_air_hockey_score)))))

(event Custom|Win
  (Development|PrintString "Give player tickets"))

(event EventBeginPlay)

(event Collision|EventActorBeginOverlap
  (params (OtherActor :type Actor%20Object%20Reference)))

(event EventTick
  (params (DeltaSeconds :type Float%20%28single-precision%29)))

(fn ConstructionScript)