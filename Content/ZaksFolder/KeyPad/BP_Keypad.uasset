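; BP_Keypad is a physical keypad that unlocks a referenced door when the correct four-digit PIN is entered.
; Digit collision components call AddDigit when a KeyPadFinger-tagged component overlaps, except 9, which requires BP_PoolCue and plays a sound.
; AddDigit appends after a short delay, then unlocks on a match or clears wrong entries; its CanPress flag is never checked.
; A separate collision volume shows and hides a widget.
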(event OnComponentBeginOverlap(0)
  (params (OverlappedComponent :type Primitive%20Component%20Object%20Reference) (OtherActor :type Actor%20Object%20Reference) (OtherComp :type Primitive%20Component%20Object%20Reference) (OtherBodyIndex :type Integer) (bFromSweep :type Boolean) (SweepResult :type Hit%20Result%20Structure%20%28by%20ref%29))
  ;[0.15 0.15 0.15 0.5] 0 Keypad
  (if (Components|ComponentHasTag OtherComp "KeyPadFinger")
    (CallFunction|AddDigit "0")))

(event OnComponentBeginOverlap(1)
  (params (OverlappedComponent :type Primitive%20Component%20Object%20Reference) (OtherActor :type Actor%20Object%20Reference) (OtherComp :type Primitive%20Component%20Object%20Reference) (OtherBodyIndex :type Integer) (bFromSweep :type Boolean) (SweepResult :type Hit%20Result%20Structure%20%28by%20ref%29))
  ;[0.15 0.15 0.15 0.5] 1 Keypad
  (if (Components|ComponentHasTag OtherComp "KeyPadFinger")
    (CallFunction|AddDigit "1")))

(event OnComponentBeginOverlap(CollisionForWidget)
  (params (OverlappedComponent :type Primitive%20Component%20Object%20Reference) (OtherActor :type Actor%20Object%20Reference) (OtherComp :type Primitive%20Component%20Object%20Reference) (OtherBodyIndex :type Integer) (bFromSweep :type Boolean) (SweepResult :type Hit%20Result%20Structure%20%28by%20ref%29))
  (Rendering|SetVisibility (Variables|Default|GetWidget) true true))

(event OnComponentEndOverlap(CollisionForWidget)
  (params (OverlappedComponent :type Primitive%20Component%20Object%20Reference) (OtherActor :type Actor%20Object%20Reference) (OtherComp :type Primitive%20Component%20Object%20Reference) (OtherBodyIndex :type Integer))
  (Rendering|SetVisibility (Variables|Default|GetWidget) false true))

(event OnComponentBeginOverlap(2)
  (params (OverlappedComponent :type Primitive%20Component%20Object%20Reference) (OtherActor :type Actor%20Object%20Reference) (OtherComp :type Primitive%20Component%20Object%20Reference) (OtherBodyIndex :type Integer) (bFromSweep :type Boolean) (SweepResult :type Hit%20Result%20Structure%20%28by%20ref%29))
  ;[0.15 0.15 0.15 0.5] 2 Keypad
  (if (Components|ComponentHasTag OtherComp "KeyPadFinger")
    (CallFunction|AddDigit "2")))

(event OnComponentBeginOverlap(3)
  (params (OverlappedComponent :type Primitive%20Component%20Object%20Reference) (OtherActor :type Actor%20Object%20Reference) (OtherComp :type Primitive%20Component%20Object%20Reference) (OtherBodyIndex :type Integer) (bFromSweep :type Boolean) (SweepResult :type Hit%20Result%20Structure%20%28by%20ref%29))
  ;[0.15 0.15 0.15 0.5] 3 Keypad
  (if (Components|ComponentHasTag OtherComp "KeyPadFinger")
    (CallFunction|AddDigit "3")))

(event OnComponentBeginOverlap(4)
  (params (OverlappedComponent :type Primitive%20Component%20Object%20Reference) (OtherActor :type Actor%20Object%20Reference) (OtherComp :type Primitive%20Component%20Object%20Reference) (OtherBodyIndex :type Integer) (bFromSweep :type Boolean) (SweepResult :type Hit%20Result%20Structure%20%28by%20ref%29))
  ;[0.15 0.15 0.15 0.5] 4 Keypad
  (if (Components|ComponentHasTag OtherComp "KeyPadFinger")
    (CallFunction|AddDigit "4")))

(event OnComponentBeginOverlap(5)
  (params (OverlappedComponent :type Primitive%20Component%20Object%20Reference) (OtherActor :type Actor%20Object%20Reference) (OtherComp :type Primitive%20Component%20Object%20Reference) (OtherBodyIndex :type Integer) (bFromSweep :type Boolean) (SweepResult :type Hit%20Result%20Structure%20%28by%20ref%29))
  ;[0.15 0.15 0.15 0.5] 5 Keypad
  (if (Components|ComponentHasTag OtherComp "KeyPadFinger")
    (CallFunction|AddDigit "5")))

(event OnComponentBeginOverlap(6)
  (params (OverlappedComponent :type Primitive%20Component%20Object%20Reference) (OtherActor :type Actor%20Object%20Reference) (OtherComp :type Primitive%20Component%20Object%20Reference) (OtherBodyIndex :type Integer) (bFromSweep :type Boolean) (SweepResult :type Hit%20Result%20Structure%20%28by%20ref%29))
  ;[0.15 0.15 0.15 0.5] 6 Keypad
  (if (Components|ComponentHasTag OtherComp "KeyPadFinger")
    (CallFunction|AddDigit "6")))

(event OnComponentBeginOverlap(7)
  (params (OverlappedComponent :type Primitive%20Component%20Object%20Reference) (OtherActor :type Actor%20Object%20Reference) (OtherComp :type Primitive%20Component%20Object%20Reference) (OtherBodyIndex :type Integer) (bFromSweep :type Boolean) (SweepResult :type Hit%20Result%20Structure%20%28by%20ref%29))
  ;[0.15 0.15 0.15 0.5] 7 Keypad
  (if (Components|ComponentHasTag OtherComp "KeyPadFinger")
    (CallFunction|AddDigit "7")))

(event OnComponentBeginOverlap(8)
  (params (OverlappedComponent :type Primitive%20Component%20Object%20Reference) (OtherActor :type Actor%20Object%20Reference) (OtherComp :type Primitive%20Component%20Object%20Reference) (OtherBodyIndex :type Integer) (bFromSweep :type Boolean) (SweepResult :type Hit%20Result%20Structure%20%28by%20ref%29))
  ;[0.15 0.15 0.15 0.5] 8 Keypad
  (if (Components|ComponentHasTag OtherComp "KeyPadFinger")
    (CallFunction|AddDigit "8")))

(event OnComponentBeginOverlap(9)
  (params (OverlappedComponent :type Primitive%20Component%20Object%20Reference) (OtherActor :type Actor%20Object%20Reference) (OtherComp :type Primitive%20Component%20Object%20Reference) (OtherBodyIndex :type Integer) (bFromSweep :type Boolean) (SweepResult :type Hit%20Result%20Structure%20%28by%20ref%29))
  ;[0.15 0.15 0.15 0.5] 9 Keypad
  (Utilities|Casting|CastToBP_PoolCue OtherActor)
  (Audio|PlaySoundatLocation "/Game/ZaksFolder/KeyPad/KeyPadSound_Cue.KeyPadSound_Cue" (Variables|/Script/Engine.SceneComponent|GetRelativeLocation (Variables|Default|GetKeypad)) "0, 0, 0" 1.0 1.0 1.9 0 0 0 0)
  (CallFunction|AddDigit "9"))

(event Custom|AddDigit
  (params (Digit :type String))
  ;[0.15 0.15 0.15 0.5] Code for correct pin and opening the door when correct
  (if (not (Variables|Default|GetUnlocked))
    (Variables|Default|SetCanPress false)
    (Utilities|FlowControl|Delay 0.2)
    (Variables|Default|SetCanPress true)
    (bind _output_get (Variables|Default|SetEnteredCode (Utilities|String|Append (Variables|Default|GetEnteredCode) Digit)))
    (Development|PrintString _output_get)
    (if (== (Utilities|String|Len (Variables|Default|GetEnteredCode)) 4)
      (if (Utilities|Enum|Equal(Enum) (Variables|Default|GetEnteredCode) (Variables|Default|GetCorrectCode))
        (Variables|Default|SetUnlocked true)
        (Development|PrintString "Correct Pin")
        (Default|UnlockDoor (Variables|Default|GetDoorRef))
        (else
          (Development|PrintString "Wrong Pin")
          (Variables|Default|SetEnteredCode ""))))))

(event EventBeginPlay)

(event Collision|EventActorBeginOverlap
  (params (OtherActor :type Actor%20Object%20Reference)))

(event EventTick
  (params (DeltaSeconds :type Float%20%28single-precision%29)))

(fn ConstructionScript)