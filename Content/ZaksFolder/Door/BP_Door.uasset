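; BP_Door is a physics-driven door that can be locked shut or left free to swing.
; On BeginPlay it applies the state set by IsDoorLocked through the DoorLocked or DoorOpen event.
; Each event updates that flag and switches the PhysicsConstraint's Swing1 limit between fully locked and a limited swing arc, so no animation is used.
; A few disconnected nodes, including a GrabComponent cast, never run.
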(event Custom|DoorLocked
  (Variables|Default|SetIsDoorLocked? true)
  (Class|PhysicsConstraintComponent|SetAngularSwing1Limit (Variables|Default|GetPhysicsConstraint) "ACM_Locked" 0.0))

(event Custom|DoorOpen
  (Variables|Default|SetIsDoorLocked? false)
  (Class|PhysicsConstraintComponent|SetAngularSwing1Limit (Variables|Default|GetPhysicsConstraint) "ACM_Limited" 1.2e+02))

(event EventBeginPlay
  (if (Variables|Default|GetIsDoorLocked?)
    (CallFunction|DoorLocked)
    (else
      (CallFunction|DoorOpen))))

(event Collision|EventActorBeginOverlap
  (params (OtherActor :type Actor%20Object%20Reference)))

(event EventTick
  (params (DeltaSeconds :type Float%20%28single-precision%29)))

(fn ConstructionScript)