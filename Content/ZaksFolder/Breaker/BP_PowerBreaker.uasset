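; Power breaker actor that switches on power when the VR pawn touches it.
; Box overlap with a VRPawn calls PowerOn, which hides the widget and plays a timeline that moves the red slider mesh along relative Z.
; When the timeline finishes, it calls PowerIsOn on the referenced power cable to pass the powered state on.
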(event OnComponentBeginOverlap(Box)
  (params (OverlappedComponent :type Primitive%20Component%20Object%20Reference) (OtherActor :type Actor%20Object%20Reference) (OtherComp :type Primitive%20Component%20Object%20Reference) (OtherBodyIndex :type Integer) (bFromSweep :type Boolean) (SweepResult :type Hit%20Result%20Structure%20%28by%20ref%29))
  (Utilities|Casting|CastToVRPawn OtherActor)
  (CallFunction|Poweron))

(event Custom|PowerOn
  (bind _sm_redslidersforbreaker (Variables|Default|GetSM_RedSlidersForBreaker))
  (bind _relativelocation (Variables|/Script/Engine.SceneComponent|GetRelativeLocation _sm_redslidersforbreaker))
  (Rendering|SetVisibility (Variables|Default|GetWidget) false true)
  (bind _slidersgoingup (Timeline|SlidersGoUp Play)
    (:Update
      (Transformation|SetRelativeLocation _sm_redslidersforbreaker (Math|Vector|MakeVector (.x _relativelocation) (.y _relativelocation) _slidersgoingup) false false))
    (:Finished
      (Default|PowerIson (Variables|Default|GetPowerCableRef)))))

(event EventBeginPlay)

(event Collision|EventActorBeginOverlap
  (params (OtherActor :type Actor%20Object%20Reference)))

(event EventTick
  (params (DeltaSeconds :type Float%20%28single-precision%29)))

(fn ConstructionScript)