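; VR arcade prize wheel that a VRPawn starts by overlapping its button, awarding a ticket once the cumulative score reaches 100.
; The press animates the button, then triggers a timeline-driven spin with a random angle offset alongside sound and flashing lights, which stop after a delay.
; When the spin finishes, DetermineScore maps the wheel's roll to ten segments, updates the score widget and re-arms the button.
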(event OnComponentBeginOverlap(SphereCollForBtn)
  (params (OverlappedComponent :type Primitive%20Component%20Object%20Reference) (OtherActor :type Actor%20Object%20Reference) (OtherComp :type Primitive%20Component%20Object%20Reference) (OtherBodyIndex :type Integer) (bFromSweep :type Boolean) (SweepResult :type Hit%20Result%20Structure%20%28by%20ref%29))
  ;[0.15 0 0.119 0.5 34] Intialisation Of Wheel
  (bind _asvrpawn (Utilities|Casting|CastToVRPawn OtherActor))
  (Variables|Default|SetVRPawnRef _asvrpawn)
  (if (not (Variables|Default|GetActive))
    (Variables|Default|SetActive true)
    (Utilities|FlowControl|Sequence
      (:then_0
        (bind _buttonpressed (Timeline|ButtonPressed Play)
          (:Update
            (Transformation|SetRelativeLocation (Variables|Default|GetSM_ButtonForWheel) _buttonpressed false false)
            (Utilities|FlowControl|Delay 1.5)
            (Timeline|ButtonPressed Reverse))))
      (:then_1
        (Utilities|FlowControl|Delay 1.0)
        (CallFunction|StartSpin))
      (:then_2
        (Utilities|FlowControl|Delay 1.0)
        (CallFunction|ArcadeShake)
        (Default|MakeNoise (Variables|Default|GetSound))))))

(event Custom|StartSpin
  (bind _wheel (Variables|Default|GetWheel))
  ;[0.15 0.15 0.15 0.5] WheelSpin
  (if (Variables|Default|GetIsSpinning?)
    (Variables|Default|SetRandom%20Result (Math|Random|RandomFloatinRange 0.0 3.6e+02))
    (bind _spin (Timeline|Timeline PlayFromStart)
      (:Update
        (Transformation|SetRelativeRotation _wheel (Math|Rotator|MakeRotator (+ (* _spin (Variables|Default|GetSpinSpeed)) (Variables|Default|GetRandom%20Result)) 0.0 0.0) false false)
        (Variables|Default|SetRelative%20Rotation%20X%20%28Roll%29 (.roll (Variables|/Script/Engine.SceneComponent|GetRelativeRotation _wheel))))
      (:Finished
        (bind _scoretoadd (CallFunction|DetermineScore (Variables|Default|GetRelative%20Rotation%20X%20%28Roll%29)))
        (Variables|Default|SetActive false)
        (bind _output_get (Variables|Default|SetScore (+ _scoretoadd (Variables|Default|GetScore))))
        (CallFunction|AddScore)
        (if (>= _output_get 100)
          (CallFunction|Win))))))

(event Custom|ArcadeShake
  (bind _pac_man_wheelspinnoise_cue (Variables|Default|GetPac-Man_WheelSpinNoise_Cue))
  ;[0.15 0.15 0.15 0.5] ArcadeShake
  (Utilities|FlowControl|Sequence
    (:then_2
      (Audio|SpawnSoundAttached "/Game/ZaksFolder/WheelSpin/Pac-Man_WheelSpinNoise_Cue.Pac-Man_WheelSpinNoise_Cue" (Variables|Default|GetMainStation) "None" "0, 0, 0" "0, 0, 0" "KeepRelativeOffset" false 0.25 1.0 0.0 0 0))
    (:then_3
      (bind _flash (Timeline|TL_ArcadeLights PlayFromStart)
        (:Update
          (Utilities|FlowControl|Sequence
            (:then_0
              (Rendering|Components|Light|SetIntensity (Variables|Default|GetPointLight_Left) (Math|Float|Lerp 0.0 1.2e+04 _flash)))
            (:then_1
              (Rendering|Components|Light|SetIntensity (Variables|Default|GetPointLight_Right) (Math|Float|Lerp 0.0 1.2e+04 _flash)))
            (:then_2
              (Rendering|Components|Light|SetIntensity (Variables|Default|GetPointLight_TopRed) (Math|Float|Lerp 0.0 1.2e+04 _flash)))
            (:then_3
              (Rendering|Components|Light|SetIntensity (Variables|Default|GetPointLight_TopBlue) (Math|Float|Lerp 0.0 1.2e+04 _flash)))
            (:then_4
              (Rendering|Components|Light|SetIntensity (Variables|Default|GetPointLight_Wheel) (Math|Float|Lerp 0.0 1.2e+04 _flash)))
            (:then_5
              (Rendering|Components|Light|SetIntensity (Variables|Default|GetPointLight_WheelRed) (Math|Float|Lerp 0.0 1.2e+04 _flash)))))))
    (:then_4
      (Utilities|FlowControl|Delay 5.0)
      (Utilities|FlowControl|Sequence
        (:then_0
          (Audio|Components|Audio|Stop _pac_man_wheelspinnoise_cue)
          (bind _leftandright (Timeline|LeftandRight Stop)
            (:Update
              (Transformation|SetRelativeLocation (Variables|Default|GetMainStation) _leftandright false false))))
        (:then_1
          (Audio|Components|Audio|Stop _pac_man_wheelspinnoise_cue)
          (bind _leftandright_2 (Timeline|Timeline_0 Stop)
            (:Update
              (Transformation|SetRelativeLocation (Variables|Default|GetMainStation) _leftandright_2 false false))))
        (:then_2
          (Utilities|FlowControl|Sequence
            (:then_0
              (Timeline|TL_ArcadeLights Stop))
            (:then_1
              (Rendering|Components|Light|SetIntensity (Variables|Default|GetPointLight_TopRed) 0.0))
            (:then_2
              (Rendering|Components|Light|SetIntensity (Variables|Default|GetPointLight_TopBlue) 0.0))
            (:then_3
              (Rendering|Components|Light|SetIntensity (Variables|Default|GetPointLight_Right) 0.0))
            (:then_4
              (Rendering|Components|Light|SetIntensity (Variables|Default|GetPointLight_Left) 0.0))
            (:then_5
              (Rendering|Components|Light|SetIntensity (Variables|Default|GetPointLight_Wheel) 0.0))
            (:then_6
              (Rendering|Components|Light|SetIntensity (Variables|Default|GetPointLight_WheelRed) 0.0))))))))

(event Custom|TestButtonPress
  (params (other%20Actor :type Character%20Object%20Reference))
  ;[0.15 0 0.119 0.5 34] Intialisation Of Wheel
)

(event Custom|AddScore
  (bind _aswbp_wheel_spin (Utilities|Casting|CastToWBP_WheelSpin (UserInterface|GetWidget (Variables|Default|GetWidget))))
  (Default|SetScore _aswbp_wheel_spin (Variables|Default|GetScore)))

(event Custom|Win
  (Default|ActivateTicket (Variables|Default|GetTicket)))

(event EventBeginPlay
  (CallFunction|TestButtonPress))

(event Collision|EventActorBeginOverlap
  (params (OtherActor :type Actor%20Object%20Reference)))

(event EventTick
  (params (DeltaSeconds :type Float%20%28single-precision%29)))

(fn ConstructionScript)

(fn DetermineScore
  (params (XRotation :type Float%20%28double-precision%29))
  (if (Math|Float|InRange(Float) XRotation -1.8e+02 -144.0 true false)
    (Variables|Default|SetScoreToAdd 5)
    (return (Variables|Default|GetScoreToAdd))
    (elif (Math|Float|InRange(Float) XRotation -144.0 -108.0 true false)
      (Variables|Default|SetScoreToAdd 20)
      (return (Variables|Default|GetScoreToAdd))
      (elif (Math|Float|InRange(Float) XRotation -108.0 -72.0 true false)
        (Variables|Default|SetScoreToAdd 40)
        (return (Variables|Default|GetScoreToAdd))
        (elif (Math|Float|InRange(Float) XRotation -72.0 -36.0 true false)
          (Variables|Default|SetScoreToAdd 5)
          (return (Variables|Default|GetScoreToAdd))
          (elif (Math|Float|InRange(Float) XRotation -36.0 0.0 true false)
            (Variables|Default|SetScoreToAdd 10)
            (return (Variables|Default|GetScoreToAdd))
            (elif (Math|Float|InRange(Float) XRotation 0.0 36.0 true false)
              (Variables|Default|SetScoreToAdd 100)
              (return (Variables|Default|GetScoreToAdd))
              (elif (Math|Float|InRange(Float) XRotation 36.0 72.0 true false)
                (Variables|Default|SetScoreToAdd 20)
                (return (Variables|Default|GetScoreToAdd))
                (elif (Math|Float|InRange(Float) XRotation 72.0 108.0 true false)
                  (Variables|Default|SetScoreToAdd 5)
                  (return (Variables|Default|GetScoreToAdd))
                  (elif (Math|Float|InRange(Float) XRotation 108.0 144.0 true false)
                    (Variables|Default|SetScoreToAdd 40)
                    (return (Variables|Default|GetScoreToAdd))
                    (elif (Math|Float|InRange(Float) XRotation 144.0 1.8e+02 true false)
                      (Variables|Default|SetScoreToAdd 10)
                      (return (Variables|Default|GetScoreToAdd)))))))))))))