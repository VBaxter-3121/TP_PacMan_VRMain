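; BP_Hammer is the hammer actor for the Whack-A-Mole game, detecting hits on moles through its box collision.
; An overlap with a BP_Mole hides that mole, then after a random delay destroys it and increments the hammer's Score.
; A DoOnce gate ignores further mole hits until that sequence finishes, and debug prints mark the hit and destruction.
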(event OnComponentBeginOverlap(BoxCollisionHammer)
  (params (OverlappedComponent :type Primitive%20Component%20Object%20Reference) (OtherActor :type Actor%20Object%20Reference) (OtherComp :type Primitive%20Component%20Object%20Reference) (OtherBodyIndex :type Integer) (bFromSweep :type Boolean) (SweepResult :type Hit%20Result%20Structure%20%28by%20ref%29))
  (bind _asbp_mole (Utilities|Casting|CastToBP_Mole OtherActor))
  (Utilities|FlowControl|DoOnce false :!label _label
    (:Completed
      (Default|HideMole _asbp_mole)
      (Development|PrintString "Mole Hit")
      (Utilities|FlowControl|Delay (Math|Random|RandomFloatinRange (Variables|Default|GetMinDelayMoleHit) (Variables|Default|GetMaxDelayMoleHit)))
      (Actor|DestroyActor _asbp_mole)
      (Variables|Default|SetScore (+ (Variables|Default|GetScore) 1))
      (Development|PrintString "Mole Destroyed")
      (goto _label Reset))))

(event EventBeginPlay
  (Collision|SetCollisionEnabled (Variables|Default|GetBoxCollisionHammer) "QueryAndPhysics"))

(event Collision|EventActorBeginOverlap
  (params (OtherActor :type Actor%20Object%20Reference)))

(event EventTick
  (params (DeltaSeconds :type Float%20%28single-precision%29)))

(fn ConstructionScript)