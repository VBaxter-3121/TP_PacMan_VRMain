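; Whack-a-mole arcade machine that runs timed rounds across five child-actor BP_Mole instances and shows state on a widget-component screen.
; StartWhackRound ignores repeat presses during a round, starts each mole's random cycle and sets the round timer.
; RegisterMoleHit adds points and updates the score text.
; EndWhackRound hides the moles, activates a ticket reward on a win or makes noise on a loss, then resets the screen after a delay.
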(event Custom|RegisterMoleHit
  ;[0.875 0.2828 0.8339 0.5] calculates score when mole is hit
  (Variables|Default|SetCurrentScore (+ (Variables|Default|GetCurrentScore) (Variables|Default|GetPointsPerMoleHit)))
  (Rendering|Components|TextRender|SetText (Variables|/Game/ChelFolder/UI/WBP_WhackAMoleScreen.WBP_WhackAMoleScreen_C|GetTxt_Score (Variables|Default|GetWhackScreenRef)) (Utilities|Text|FormatText "SCORE:{Score}" (Utilities|Text|ToText(Integer) (Variables|Default|GetCurrentScore) false false))))

(event Custom|StartWhackRound
  ;[0.8813 0.415 0.8854 0.5] This starts the round only one time and prevents the round from being restarted by button press
  (if (not (Variables|Default|GetIsRoundActive))
    (Variables|Default|SetIsRoundActive true)
    (Variables|Default|SetCurrentScore 0)
    (Widget|SetVisibility (Variables|/Game/ChelFolder/UI/WBP_WhackAMoleScreen.WBP_WhackAMoleScreen_C|GetTxt_PressButton (Variables|Default|GetWhackScreenRef)) "Hidden")
    (Widget|SetVisibility (Variables|/Game/ChelFolder/UI/WBP_WhackAMoleScreen.WBP_WhackAMoleScreen_C|GetTxt_Score (Variables|Default|GetWhackScreenRef)) "Visible")
    (Widget|SetVisibility (Variables|/Game/ChelFolder/UI/WBP_WhackAMoleScreen.WBP_WhackAMoleScreen_C|GetTxt_Win (Variables|Default|GetWhackScreenRef)) "Hidden")
    (Widget|SetVisibility (Variables|/Game/ChelFolder/UI/WBP_WhackAMoleScreen.WBP_WhackAMoleScreen_C|GetTxt_GameOver (Variables|Default|GetWhackScreenRef)) "Hidden")
    (Utilities|FlowControl|Sequence
      (:then_0
        (bind _asbp_mole (Utilities|Casting|CastToBP_Mole (Variables|/Script/Engine.ChildActorComponent|GetChildActor (Variables|Default|GetBP_Mole_C_1))))
        (Default|StartRandomCycle _asbp_mole))
      (:then_1
        (bind _asbp_mole_2 (Utilities|Casting|CastToBP_Mole (Variables|/Script/Engine.ChildActorComponent|GetChildActor (Variables|Default|GetBP_Mole_C_2))))
        (Default|StartRandomCycle _asbp_mole_2))
      (:then_2
        (bind _asbp_mole_3 (Utilities|Casting|CastToBP_Mole (Variables|/Script/Engine.ChildActorComponent|GetChildActor (Variables|Default|GetBP_Mole_C_3))))
        (Default|StartRandomCycle _asbp_mole_3))
      (:then_3
        (bind _asbp_mole_4 (Utilities|Casting|CastToBP_Mole (Variables|/Script/Engine.ChildActorComponent|GetChildActor (Variables|Default|GetBP_Mole_C_4))))
        (Default|StartRandomCycle _asbp_mole_4))
      (:then_4
        (bind _asbp_mole_5 (Utilities|Casting|CastToBP_Mole (Variables|/Script/Engine.ChildActorComponent|GetChildActor (Variables|Default|GetBP_Mole_C_5))))
        (Default|StartRandomCycle _asbp_mole_5))
      (:then_5
        (Utilities|Time|SetTimerbyEvent (EventDispatchers|CreateEvent :!event Custom|EndWhackRound) (Variables|Default|GetRoundTimer))))))

(event Custom|EndWhackRound
  ;[0.3564 0.1714 0.3613] Ends Whackround
  (Variables|Default|SetIsRoundActive false)
  (Utilities|FlowControl|Sequence
    (:then_0
      (bind _asbp_mole (Utilities|Casting|CastToBP_Mole (Variables|/Script/Engine.ChildActorComponent|GetChildActor (Variables|Default|GetBP_Mole_C_1))))
      (Default|HideMole _asbp_mole))
    (:then_1
      (bind _asbp_mole_2 (Utilities|Casting|CastToBP_Mole (Variables|/Script/Engine.ChildActorComponent|GetChildActor (Variables|Default|GetBP_Mole_C_2))))
      (Default|HideMole _asbp_mole_2))
    (:then_2
      (bind _asbp_mole_3 (Utilities|Casting|CastToBP_Mole (Variables|/Script/Engine.ChildActorComponent|GetChildActor (Variables|Default|GetBP_Mole_C_3))))
      (Default|HideMole _asbp_mole_3))
    (:then_3
      (bind _asbp_mole_4 (Utilities|Casting|CastToBP_Mole (Variables|/Script/Engine.ChildActorComponent|GetChildActor (Variables|Default|GetBP_Mole_C_4))))
      (Default|HideMole _asbp_mole_4))
    (:then_4
      (bind _asbp_mole_5 (Utilities|Casting|CastToBP_Mole (Variables|/Script/Engine.ChildActorComponent|GetChildActor (Variables|Default|GetBP_Mole_C_5))))
      (Default|HideMole _asbp_mole_5))
    (:then_5
      (if (>= (Variables|Default|GetCurrentScore) (Variables|Default|GetScoreNeededToWin))
        (Widget|SetVisibility (Variables|/Game/ChelFolder/UI/WBP_WhackAMoleScreen.WBP_WhackAMoleScreen_C|GetTxt_Win (Variables|Default|GetWhackScreenRef)) "Visible")
        (Widget|SetVisibility (Variables|/Game/ChelFolder/UI/WBP_WhackAMoleScreen.WBP_WhackAMoleScreen_C|GetTxt_GameOver (Variables|Default|GetWhackScreenRef)) "Hidden")
        (Widget|SetVisibility (Variables|/Game/ChelFolder/UI/WBP_WhackAMoleScreen.WBP_WhackAMoleScreen_C|GetTxt_Score (Variables|Default|GetWhackScreenRef)) "Hidden")
        (Widget|SetVisibility (Variables|/Game/ChelFolder/UI/WBP_WhackAMoleScreen.WBP_WhackAMoleScreen_C|GetTxt_PressButton (Variables|Default|GetWhackScreenRef)) "Hidden")
        (Default|ActivateTicket (Variables|Default|GetWhackTicketRewardRef))
        (Utilities|FlowControl|Delay 3.0)
        (CallFunction|ResetWhackScreen)
        (else
          (Default|MakeNoise (Variables|Default|GetNoise))
          (Widget|SetVisibility (Variables|/Game/ChelFolder/UI/WBP_WhackAMoleScreen.WBP_WhackAMoleScreen_C|GetTxt_Win (Variables|Default|GetWhackScreenRef)) "Hidden")
          (Widget|SetVisibility (Variables|/Game/ChelFolder/UI/WBP_WhackAMoleScreen.WBP_WhackAMoleScreen_C|GetTxt_GameOver (Variables|Default|GetWhackScreenRef)) "Visible")
          (Widget|SetVisibility (Variables|/Game/ChelFolder/UI/WBP_WhackAMoleScreen.WBP_WhackAMoleScreen_C|GetTxt_PressButton (Variables|Default|GetWhackScreenRef)) "Hidden")
          (Widget|SetVisibility (Variables|/Game/ChelFolder/UI/WBP_WhackAMoleScreen.WBP_WhackAMoleScreen_C|GetTxt_Score (Variables|Default|GetWhackScreenRef)) "Hidden")
          (Utilities|FlowControl|Delay 2.0)
          (CallFunction|ResetWhackScreen))))))

(event Custom|ResetWhackScreen
  (Widget|SetVisibility (Variables|/Game/ChelFolder/UI/WBP_WhackAMoleScreen.WBP_WhackAMoleScreen_C|GetTxt_PressButton (Variables|Default|GetWhackScreenRef)) "Visible")
  (Widget|SetVisibility (Variables|/Game/ChelFolder/UI/WBP_WhackAMoleScreen.WBP_WhackAMoleScreen_C|GetTxt_Score (Variables|Default|GetWhackScreenRef)) "Hidden")
  (Widget|SetVisibility (Variables|/Game/ChelFolder/UI/WBP_WhackAMoleScreen.WBP_WhackAMoleScreen_C|GetTxt_Win (Variables|Default|GetWhackScreenRef)) "Hidden")
  (Widget|SetVisibility (Variables|/Game/ChelFolder/UI/WBP_WhackAMoleScreen.WBP_WhackAMoleScreen_C|GetTxt_GameOver (Variables|Default|GetWhackScreenRef)) "Hidden")
  (Rendering|Components|TextRender|SetText (Variables|/Game/ChelFolder/UI/WBP_WhackAMoleScreen.WBP_WhackAMoleScreen_C|GetTxt_Score (Variables|Default|GetWhackScreenRef)) (Utilities|Text|FormatText "SCORE: {0}" (Utilities|Text|ToText(Integer) 0 false false))))

(event EventBeginPlay
  (bind _aswbp_whack_amole_screen (Utilities|Casting|CastToWBP_WhackAMoleScreen (UserInterface|GetUserWidgetObject (Variables|Default|GetWhackScreenWidget))))
  (Variables|Default|SetWhackScreenRef _aswbp_whack_amole_screen)
  (Widget|SetVisibility (Variables|/Game/ChelFolder/UI/WBP_WhackAMoleScreen.WBP_WhackAMoleScreen_C|GetTxt_PressButton (Variables|Default|GetWhackScreenRef)) "Visible")
  (Widget|SetVisibility (Variables|/Game/ChelFolder/UI/WBP_WhackAMoleScreen.WBP_WhackAMoleScreen_C|GetTxt_Score (Variables|Default|GetWhackScreenRef)) "Hidden")
  (Widget|SetVisibility (Variables|/Game/ChelFolder/UI/WBP_WhackAMoleScreen.WBP_WhackAMoleScreen_C|GetTxt_Win (Variables|Default|GetWhackScreenRef)) "Hidden")
  (Widget|SetVisibility (Variables|/Game/ChelFolder/UI/WBP_WhackAMoleScreen.WBP_WhackAMoleScreen_C|GetTxt_GameOver (Variables|Default|GetWhackScreenRef)) "Hidden"))

(fn ConstructionScript)