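; Mole actor for a Whack-A-Mole game that pops its mesh up and hides it again on a random cycle.
; BeginPlay caches the hidden and raised Z positions, then random-delay timers alternate playing and reversing the BopUpAndDown timeline, which lerps the mesh height.
; MoleHit reverses a separate DestroyMole timeline that drives the same height lerp, without clearing the cycle's timers.
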(event Custom|StartRandomCycle
  (Utilities|Time|SetTimerbyEvent (delegate Custom|PopUp) (Math|Random|RandomFloatinRange (Variables|Default|GetMinWaitTime) (Variables|Default|GetMaxWaitTime))))

(event Custom|PopUp
  (bind _sm_mole (Variables|Default|GetSM_Mole))
  (bind _relativelocation (Variables|/Script/Engine.SceneComponent|GetRelativeLocation _sm_mole))
  (bind (_direction _alpha) (Timeline|BopUpAndDown Play)
    (:Update
      (Transformation|SetRelativeLocation _sm_mole (Math|Vector|MakeVector (.x _relativelocation) (.y _relativelocation) (Math|Float|Lerp (Variables|Default|GetHidden) (Variables|Default|GetUp) _alpha)) false false))
    (:Finished
      (switch Utilities|FlowControl|Switch|SwitchonETimelineDirection _direction
        (:Forward
          (Utilities|Time|SetTimerbyEvent (delegate Custom|HideMole) (Math|Random|RandomFloatinRange (Variables|Default|GetMinUpTime) (Variables|Default|GetMaxUpTime))))
        (:Backward
          (CallFunction|StartRandomCycle))))))

(event Custom|HideMole
  (bind _sm_mole (Variables|Default|GetSM_Mole))
  (bind _relativelocation (Variables|/Script/Engine.SceneComponent|GetRelativeLocation _sm_mole))
  (bind (_direction _alpha) (Timeline|BopUpAndDown Reverse)
    (:Update
      (Transformation|SetRelativeLocation _sm_mole (Math|Vector|MakeVector (.x _relativelocation) (.y _relativelocation) (Math|Float|Lerp (Variables|Default|GetHidden) (Variables|Default|GetUp) _alpha)) false false))
    (:Finished
      (switch Utilities|FlowControl|Switch|SwitchonETimelineDirection _direction
        (:Forward
          (Utilities|Time|SetTimerbyEvent (delegate Custom|HideMole) (Math|Random|RandomFloatinRange (Variables|Default|GetMinUpTime) (Variables|Default|GetMaxUpTime))))
        (:Backward
          (CallFunction|StartRandomCycle))))))

(event Custom|MoleHit
  (bind _sm_mole (Variables|Default|GetSM_Mole))
  (bind _relativelocation (Variables|/Script/Engine.SceneComponent|GetRelativeLocation _sm_mole))
  (bind _newtrack_0 (Timeline|Destroy%20Mole Reverse)
    (:Update
      (Transformation|SetRelativeLocation _sm_mole (Math|Vector|MakeVector (.x _relativelocation) (.y _relativelocation) (Math|Float|Lerp (Variables|Default|GetHidden) (Variables|Default|GetUp) _newtrack_0)) false false))))

(event EventBeginPlay
  (bind _sm_mole (Variables|Default|GetSM_Mole))
  (bind _relativelocation (Variables|/Script/Engine.SceneComponent|GetRelativeLocation _sm_mole))
  (bind _z (Math|Vector|BreakVector _relativelocation))
  (Variables|Default|SetHidden _z)
  (Variables|Default|SetUp (+ _z (Variables|Default|GetMoveAmount)))
  (CallFunction|StartRandomCycle))

(event Collision|EventActorBeginOverlap
  (params (OtherActor :type Actor%20Object%20Reference)))

(event EventTick
  (params (DeltaSeconds :type Float%20%28single-precision%29)))

(fn ConstructionScript)